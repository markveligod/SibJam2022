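; BP_TriggerWin is a trigger actor that lets the player win the game by interacting inside its box.
; When a BP_BaseCharacter overlaps the box, it shows a widget, stores the character and binds to its GamePlayerController's OnInteract dispatcher.
; Interacting tells BP_SibJamp2022GameMode to change the game state to GameWin.
; Leaving the box hides the widget, which also starts hidden, and unbinds the interact event.
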(event OnComponentBeginOverlap(Box)
  (params (OverlappedComponent :type Primitive%20Component%20Object%20Reference) (OtherActor :type Actor%20Object%20Reference) (OtherComp :type Primitive%20Component%20Object%20Reference) (OtherBodyIndex :type Integer) (bFromSweep :type Boolean) (SweepResult :type Hit%20Result%20Structure%20%28by%20ref%29))
  (bind _asbp_base_character (Utilities|Casting|CastToBP_BaseCharacter OtherActor))
  (Variables|Default|SetCharRef _asbp_base_character)
  (bind _asgame_player_controller (Utilities|Casting|CastToGamePlayerController (Pawn|GetController _asbp_base_character)))
  (EventDispatchers|AssignOnInteract _asgame_player_controller (delegate Custom|OnInteract_Event_0))
  (Rendering|SetVisibility (Variables|Default|GetWidget) true false))

(event OnComponentEndOverlap(Box)
  (params (OverlappedComponent :type Primitive%20Component%20Object%20Reference) (OtherActor :type Actor%20Object%20Reference) (OtherComp :type Primitive%20Component%20Object%20Reference) (OtherBodyIndex :type Integer))
  (Utilities|Casting|CastToBP_BaseCharacter OtherActor)
  (Rendering|SetVisibility (Variables|Default|GetWidget) false false)
  (bind _asgame_player_controller (Utilities|Casting|CastToGamePlayerController (Pawn|GetController (Variables|Default|GetCharRef))))
  (EventDispatchers|UnbindEventfromOnInteract _asgame_player_controller (delegate Custom|OnInteract_Event_0)))

(event Custom|OnInteract_Event_0
  (bind _asbp_sib_jamp_2022game_mode (Utilities|Casting|CastToBP_SibJamp2022GameMode (Game|GetGameMode)))
  (Class|SibJamp2022ProjectGameModeBase|ChangeGameState _asbp_sib_jamp_2022game_mode "GameWin"))

(event EventBeginPlay
  (Rendering|SetVisibility (Variables|Default|GetWidget) false false))

(fn ConstructionScript)