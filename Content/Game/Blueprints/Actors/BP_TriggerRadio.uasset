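; Interactive radio trigger that plays a one-shot sound when the player interacts inside its box.
; Overlap by BP_BaseCharacter shows a widget, starts the Radio audio and binds the player controller's OnInteract; leaving reverses all three.
; Interacting stops Radio, plays SoundToPlay in 2D and passes its duration to WBP_Game from the HUD's widget map.
; IsPlay blocks replays and clears after that duration, only if the game widget was found.
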(event OnComponentBeginOverlap(Box)
  (params (OverlappedComponent :type Primitive%20Component%20Object%20Reference) (OtherActor :type Actor%20Object%20Reference) (OtherComp :type Primitive%20Component%20Object%20Reference) (OtherBodyIndex :type Integer) (bFromSweep :type Boolean) (SweepResult :type Hit%20Result%20Structure%20%28by%20ref%29))
  (bind _asbp_base_character (Utilities|Casting|CastToBP_BaseCharacter OtherActor))
  (Variables|Default|SetCharRef _asbp_base_character)
  (bind _asgame_player_controller (Utilities|Casting|CastToGamePlayerController (Pawn|GetController _asbp_base_character)))
  (EventDispatchers|AssignOnInteract _asgame_player_controller (delegate Custom|OnInteractEvent))
  (Rendering|SetVisibility (Variables|Default|GetWidget) true false)
  (Audio|Components|Audio|Play (Variables|Default|Getradio) 0.0))

(event OnComponentEndOverlap(Box)
  (params (OverlappedComponent :type Primitive%20Component%20Object%20Reference) (OtherActor :type Actor%20Object%20Reference) (OtherComp :type Primitive%20Component%20Object%20Reference) (OtherBodyIndex :type Integer))
  (Utilities|Casting|CastToBP_BaseCharacter OtherActor)
  (Rendering|SetVisibility (Variables|Default|GetWidget) false false)
  (bind _asgame_player_controller (Utilities|Casting|CastToGamePlayerController (Pawn|GetController (Variables|Default|GetCharRef))))
  (EventDispatchers|UnbindEventfromOnInteract _asgame_player_controller (delegate Custom|OnInteractEvent))
  (Audio|Components|Audio|Stop (Variables|Default|Getradio)))

(event Custom|OnInteractEvent
  (bind _soundtoplay (Variables|ActorSettings|GetSoundToPlay))
  (bind _duration (Variables|/Script/Engine.SoundBase|GetDuration _soundtoplay))
  (if (not (Variables|Default|GetIsPlay))
    (Audio|Components|Audio|Stop (Variables|Default|Getradio))
    (Utilities|IsValid (Variables|ActorSettings|GetSoundToPlay)
      (:Is%20Valid
        (Variables|Default|SetIsPlay true)
        (Audio|PlaySound2D (Variables|ActorSettings|GetSoundToPlay) 1.0 1.0 0.0 0 0)
        (bind _asbp_game_player_controller (Utilities|Casting|CastToBP_GamePlayerController (Pawn|GetController (Variables|Default|GetCharRef))))
        (bind _asgame_jam_hud (Utilities|Casting|CastToGameJamHUD (HUD|GetHUD _asbp_game_player_controller)))
        (if (.ReturnValue (Utilities|Map|Find (Class|GameJamHUD|GetRepoWidgets _asgame_jam_hud) "GameProgress"))
          (bind _aswbp_game (Utilities|Casting|CastToWBP_Game (.Value (Utilities|Map|Find (Class|GameJamHUD|GetRepoWidgets _asgame_jam_hud) "GameProgress"))))
          (Default|RadioEvent _aswbp_game _duration)
          (Utilities|FlowControl|Delay _duration)
          (Variables|Default|SetIsPlay false))))))

(event EventBeginPlay
  (Rendering|SetVisibility (Variables|Default|GetWidget) false false)
  (Audio|Components|Audio|Stop (Variables|Default|Getradio)))

(fn ConstructionScript)