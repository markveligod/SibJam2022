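; Interactive climbable rope that a BP_BaseCharacter can grab and release through the player controller's interact event.
; Capsule overlap shows a prompt widget and binds that event; interacting while climbing, or leaving the capsule, releases the climb and unbinds it.
; Grabbing enables rope climbing and, if the character is below the capsule center, eases them beside the rope and turns them according to GrabRight.
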(event OnComponentBeginOverlap(Capsule)
  (params (OverlappedComponent :type Primitive%20Component%20Object%20Reference) (OtherActor :type Actor%20Object%20Reference) (OtherComp :type Primitive%20Component%20Object%20Reference) (OtherBodyIndex :type Integer) (bFromSweep :type Boolean) (SweepResult :type Hit%20Result%20Structure%20%28by%20ref%29))
  (bind _asbp_base_character (Utilities|Casting|CastToBP_BaseCharacter OtherActor))
  (Variables|Default|SetCharRef _asbp_base_character)
  (bind _asgame_player_controller (Utilities|Casting|CastToGamePlayerController (Pawn|GetController _asbp_base_character)))
  (EventDispatchers|AssignOnInteract _asgame_player_controller (EventDispatchers|CreateEvent :!event Custom|OnInteract_Event_0))
  (Rendering|SetVisibility (Variables|Default|GetWidget) true false))

(event OnComponentEndOverlap(Capsule)
  (params (OverlappedComponent :type Primitive%20Component%20Object%20Reference) (OtherActor :type Actor%20Object%20Reference) (OtherComp :type Primitive%20Component%20Object%20Reference) (OtherBodyIndex :type Integer))
  (bind _charref (Variables|Default|GetCharRef))
  (Utilities|Casting|CastToBP_BaseCharacter OtherActor)
  (Variables|/Game/Game/Blueprints/BP_BaseCharacter.BP_BaseCharacter_C|SetcanRopeUp _charref false)
  (Default|ReleaseClimbUp _charref)
  (Rendering|SetVisibility (Variables|Default|GetWidget) false false)
  (bind _asgame_player_controller (Utilities|Casting|CastToGamePlayerController (Pawn|GetController _charref)))
  (EventDispatchers|UnbindEventfromOnInteract _asgame_player_controller (EventDispatchers|CreateEvent :!event Custom|OnInteract_Event_0)))

(event Custom|OnInteract_Event_0
  (bind _cylinder (Variables|Default|GetCylinder))
  (bind _charref (Variables|Default|GetCharRef))
  (bind _charref_2 (Variables|Default|GetCharRef))
  (bind _charref_3 (Variables|Default|GetCharRef))
  (bind _charref_4 (Variables|Default|GetCharRef))
  (bind _capsule (Variables|Default|GetCapsule))
  (bind _charref_5 (Variables|Default|GetCharRef))
  (bind _returnvalue (Transformation|GetWorldLocation _capsule))
  (bind _returnvalue_2 (Transformation|GetWorldScale _cylinder))
  (bind _charactermovement (Variables|/Script/Engine.Character|GetCharacterMovement _charref_2))
  (bind _capsulecomponent (Variables|/Script/Engine.Character|GetCapsuleComponent _charref_4))
  (bind _capsulecomponent_2 (Variables|/Script/Engine.Character|GetCapsuleComponent _charref_5))
  (bind _returnvalue_3 (* (.z _returnvalue_2) 1e+02))
  (bind _returnvalue_4 (/ _returnvalue_3 2.0))
  (bind _returnvalue_5 (+ _returnvalue_4 1.2e+02))
  (if (Variables|/Game/Game/Blueprints/BP_BaseCharacter.BP_BaseCharacter_C|GetisRopeClimbing _charref_3)
    (Variables|/Game/Game/Blueprints/BP_BaseCharacter.BP_BaseCharacter_C|SetcanRopeUp _charref false)
    (Default|ReleaseClimbUp _charref)
    (Rendering|SetVisibility (Variables|Default|GetWidget) false false)
    (bind _asgame_player_controller (Utilities|Casting|CastToGamePlayerController (Pawn|GetController _charref)))
    (EventDispatchers|UnbindEventfromOnInteract _asgame_player_controller (EventDispatchers|CreateEvent :!event Custom|OnInteract_Event_0))
    (else
      (Variables|/Game/Game/Blueprints/BP_BaseCharacter.BP_BaseCharacter_C|SetcanRopeUp _charref_3 true)
      (if (Variables|Default|GetgrabRight)
        (Variables|Default|SetstepOnRope -15.0)
        (else
          (Variables|Default|SetstepOnRope 15.0)))
      (if (< (.z (Transformation|GetWorldLocation (Variables|/Script/Engine.Character|GetCapsuleComponent (Variables|Default|GetCharRef)))) (.z (Transformation|GetWorldLocation (Variables|Default|GetCapsule))))
        (Pawn|Components|CharacterMovement|SetMovementMode _charactermovement "MOVE_Falling" 0)
        (Components|Movement|StopMovementImmediately _charactermovement)
        (Components|MoveComponentTo _capsulecomponent (Math|Vector|MakeVector (.x _returnvalue) (+ (.y _returnvalue) (Variables|Default|GetstepOnRope)) (+ (- (.z (Transformation|GetWorldLocation _capsulecomponent)) _returnvalue_5) _returnvalue_5)) "0, 0, 0" true true 0.5 false)
        (if (Variables|Default|GetgrabRight)
          (Transformation|SetWorldRotation _capsulecomponent_2 "0.000000,90.000000,0.000000" false false)
          (else
            (Transformation|SetWorldRotation _capsulecomponent_2 "0.000000,-90.000000,0.000000" false false)))))))

(event EventBeginPlay
  (Rendering|SetVisibility (Variables|Default|GetWidget) false false))

(fn ConstructionScript)