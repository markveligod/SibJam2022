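; BP_StairsClimb is an interactive stair trigger that lets a BP_BaseCharacter climb using its rope-climb state.
; Overlapping the Box shows a prompt widget and binds to the GamePlayerController's OnInteract.
; Interacting toggles climbing; from below the Box it also sets Flying and eases the capsule to a hard-coded X and the Box's Y, facing a fixed direction.
; Leaving the Box or interacting while climbing releases the climb and unbinds the event.
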(event OnComponentBeginOverlap(Box)
  (params (OverlappedComponent :type Primitive%20Component%20Object%20Reference) (OtherActor :type Actor%20Object%20Reference) (OtherComp :type Primitive%20Component%20Object%20Reference) (OtherBodyIndex :type Integer) (bFromSweep :type Boolean) (SweepResult :type Hit%20Result%20Structure%20%28by%20ref%29))
  (bind _asbp_base_character (Utilities|Casting|CastToBP_BaseCharacter OtherActor))
  (bind _output_get (Variables|Default|SetCharRef _asbp_base_character))
  (Rendering|SetVisibility (Variables|Default|GetWidget) true false)
  (bind _asgame_player_controller (Utilities|Casting|CastToGamePlayerController (Pawn|GetController _output_get)))
  (EventDispatchers|AssignOnInteract _asgame_player_controller (EventDispatchers|CreateEvent :!event Custom|OnInteract_event))
  (Rendering|SetVisibility (Variables|Default|GetWidget) true false))

(event OnComponentEndOverlap(Box)
  (params (OverlappedComponent :type Primitive%20Component%20Object%20Reference) (OtherActor :type Actor%20Object%20Reference) (OtherComp :type Primitive%20Component%20Object%20Reference) (OtherBodyIndex :type Integer))
  (bind _charref (Variables|Default|GetCharRef))
  (Utilities|Casting|CastToBP_BaseCharacter OtherActor)
  (Variables|/Game/Game/Blueprints/BP_BaseCharacter.BP_BaseCharacter_C|SetcanRopeUp _charref false)
  (Variables|/Game/Game/Blueprints/BP_BaseCharacter.BP_BaseCharacter_C|SetonStairs _charref false)
  (Default|ReleaseClimbUp _charref)
  (Rendering|SetVisibility (Variables|Default|GetWidget) false false)
  (bind _asgame_player_controller (Utilities|Casting|CastToGamePlayerController (Pawn|GetController _charref)))
  (EventDispatchers|UnbindEventfromOnInteract _asgame_player_controller (EventDispatchers|CreateEvent :!event Custom|OnInteract_event)))

(event Custom|OnInteract_event
  (bind _charref (Variables|Default|GetCharRef))
  (bind _charref_2 (Variables|Default|GetCharRef))
  (bind _charref_3 (Variables|Default|GetCharRef))
  (bind _charref_4 (Variables|Default|GetCharRef))
  (bind _charactermovement (Variables|/Script/Engine.Character|GetCharacterMovement _charref_2))
  (bind _capsulecomponent (Variables|/Script/Engine.Character|GetCapsuleComponent _charref_4))
  (Components|Movement|StopMovementImmediately (Variables|/Script/Engine.Character|GetCharacterMovement _charref_3))
  (if (Variables|/Game/Game/Blueprints/BP_BaseCharacter.BP_BaseCharacter_C|GetisRopeClimbing _charref_3)
    (Variables|/Game/Game/Blueprints/BP_BaseCharacter.BP_BaseCharacter_C|SetcanRopeUp _charref false)
    (Variables|/Game/Game/Blueprints/BP_BaseCharacter.BP_BaseCharacter_C|SetonStairs _charref false)
    (Default|ReleaseClimbUp _charref)
    (Rendering|SetVisibility (Variables|Default|GetWidget) false false)
    (bind _asgame_player_controller (Utilities|Casting|CastToGamePlayerController (Pawn|GetController _charref)))
    (EventDispatchers|UnbindEventfromOnInteract _asgame_player_controller (EventDispatchers|CreateEvent :!event Custom|OnInteract_event))
    (else
      (Variables|/Game/Game/Blueprints/BP_BaseCharacter.BP_BaseCharacter_C|SetcanRopeUp _charref_3 true)
      (Variables|/Game/Game/Blueprints/BP_BaseCharacter.BP_BaseCharacter_C|SetonStairs _charref_3 true)
      (if (< (.z (Transformation|GetWorldLocation (Variables|/Script/Engine.Character|GetCapsuleComponent (Variables|Default|GetCharRef)))) (.z (Transformation|GetWorldLocation (Variables|Default|GetBox))))
        (Pawn|Components|CharacterMovement|SetMovementMode _charactermovement "MOVE_Flying" 0)
        (Components|Movement|StopMovementImmediately _charactermovement)
        (Components|MoveComponentTo _capsulecomponent (Math|Vector|MakeVector -1.49e+03 (.y (Transformation|GetWorldLocation (Variables|Default|GetBox))) (.z (Transformation|GetWorldLocation _capsulecomponent))) "0,180.000000,0.000000" true true 0.5 false)
        (Transformation|SetActorRotation _charref_4 "0,180.000000, 0")
        (Rendering|SetVisibility (Variables|Default|GetWidget) false false)))))

(event EventBeginPlay
  ;[1 1 1] Set widget invis on begin play
  (Rendering|SetVisibility (Variables|Default|GetWidget) false false))

(fn ConstructionScript)